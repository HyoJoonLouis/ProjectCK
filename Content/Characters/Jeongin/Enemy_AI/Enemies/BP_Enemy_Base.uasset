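; Base enemy character that provides chase, melee attack, sword wielding, patrol route and movement speed functions.
; ChasePlayer moves to the player, triggers Attack on arrival and repeats after a delay, with no retry on failed moves.
; Attack plays a montage and fires OnAttackEnd on completion or interruption; WieldSword attaches a spawned BP_Sword to the hand socket.
; SetMovementSpeed maps speed states to walk speeds, and GetPatrolRoute exposes the route; BeginPlay does nothing.
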(event Custom|ChasePlayer
  (AI|AIMoveTo self "0, 0, 0" (Game|GetPlayerCharacter 0) 1e+02 false
    (:OnSuccess
      (CallFunction|Attack)
      (Utilities|FlowControl|Delay 2.0)
      (CallFunction|ChasePlayer))))

(event Custom|Attack
  (Animation|Montage|PlayMontage (Variables|Character|GetMesh) "/Game/Characters/NPC/Enemy/MeleeEnemy/StandingMeleeAttackHorizontal_UE_Montage.StandingMeleeAttackHorizontal_UE_Montage"
    (:OnCompleted
      _)
    (:OnInterrupted
      _))
  (Default|CallOnAttackEnd))

(event Custom|WieldSword
  (bind _returnvalue (Game|SpawnActorfromClass "/Game/Characters/Jeongin/Weapon/BP_Sword.BP_Sword_C" (Transformation|GetActorTransform) "Undefined" "MultiplyWithRoot" 0 0))
  (Transformation|AttachComponentToComponent _returnvalue (Variables|Character|GetMesh) "hand_r_sword_socket" "SnapToTarget" "SnapToTarget" "SnapToTarget" true)
  (Variables|Default|SetIsWiedingSword true))

(event EventBeginPlay)

(fn ConstructionScript)

(fn GetPatrolRoute
  (return (Variables|AI|GetPatrolRoute)))

(fn SetMovementSpeed
  (params (Speed :type E_MovementSpeed%20Enum :default "NewEnumerator0"))
  (bind _output_get (Variables|/Script/Engine.CharacterMovementComponent|SetMaxWalkSpeed (Variables|Character|GetCharacterMovement) (Utilities|Select :Index Speed :NewEnumerator0 0.0 :NewEnumerator1 1e+02 :NewEnumerator2 3e+02 :NewEnumerator3 5e+02)))
  (return _output_get))